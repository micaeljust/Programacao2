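; BP_LevelMiniGameStar is the player-controlled star in a Flappy Bird-style level mini-game with moving pipes.
; Space bar gives the star an upward velocity impulse, enables its gravity and sets the pipes moving.
; Hitting a component tagged KillStar or Victory calls OnFinished with the result, destroys the star and stops the pipes.
; That result also goes to every BP_LevelStreamingMiniGame actor through FinishMiniGame.
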(event `self.ReceiveBeginPlay`
  (`parent.ReceiveBeginPlay`)
  (`self.EnableInput` (`GameplayStatics.GetPlayerController` 0)))

(event `Key|SpaceBar`
  (params (Key :type "Key Structure"))
  (:`Pressed`
    (`PrimitiveComponent.AddImpulse` (`self.Star`) (0.0 0.0 800.0) "None" true)
    (`PrimitiveComponent.SetEnableGravity` (`self.Star`) true)
    (set `self.IsMoving` true)
    (set `/Game/MiniGameExample/Blueprints/LevelMiniGame/BP_Pipes.IsMoving` true (`self.Pipes`))))

(event `self.ReceiveTick`
  (params (DeltaSeconds :type "Float (single-precision)")))

(event `self.Star.OnClicked`
  (params (TouchedComponent :type "PrimitiveComponent Object Reference") (ButtonPressed :type "Key Structure")))

(event `self.Star.OnComponentHit`
  (params (HitComponent :type "PrimitiveComponent Object Reference") (OtherActor :type "Actor Object Reference") (OtherComp :type "PrimitiveComponent Object Reference") (NormalImpulse :type "Vector Structure") (Hit :type "HitResult Structure (by ref)"))
  (if (`ActorComponent.ComponentHasTag` OtherComp "KillStar")
    (`self.OnFinished` false)
    (`KismetSystemLibrary.PrintString` "LOST")
    (`self.K2_DestroyActor`)
    (set `/Game/MiniGameExample/Blueprints/LevelMiniGame/BP_Pipes.IsMoving` false (`self.Pipes`))
    (bind _outactors (`GameplayStatics.GetAllActorsOfClass` "/Game/MiniGameExample/Blueprints/LevelMiniGame/BP_LevelStreamingMiniGame.BP_LevelStreamingMiniGame_C"))
    (for _array_element _outactors
      (`/Game/MiniGameExample/Blueprints/LevelMiniGame/BP_LevelStreamingMiniGame.FinishMiniGame` _array_element false))
    (elif (`ActorComponent.ComponentHasTag` OtherComp "Victory")
      (`self.OnFinished` true)
      (`KismetSystemLibrary.PrintString` "WON")
      (`self.K2_DestroyActor`)
      (set `/Game/MiniGameExample/Blueprints/LevelMiniGame/BP_Pipes.IsMoving` false (`self.Pipes`))
      (bind _outactors_2 (`GameplayStatics.GetAllActorsOfClass` "/Game/MiniGameExample/Blueprints/LevelMiniGame/BP_LevelStreamingMiniGame.BP_LevelStreamingMiniGame_C"))
      (for _array_element_2 _outactors_2
        (`/Game/MiniGameExample/Blueprints/LevelMiniGame/BP_LevelStreamingMiniGame.FinishMiniGame` _array_element_2 true)))))

(fn `UserConstructionScript`)