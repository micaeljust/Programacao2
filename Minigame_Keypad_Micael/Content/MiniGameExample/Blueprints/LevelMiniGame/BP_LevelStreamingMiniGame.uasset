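; BP_LevelStreamingMiniGame is an example mini-game that runs inside a level spawned as an actor.
; On begin, it adds a HUD widget, spawns BP_L_LevelMiniGame at a fixed raised location and disables input on the player's controlled pawn.
; On finish, it reports success or failure, destroys itself and the spawned level, removes the HUD and re-enables pawn input.
; Despite the name, it uses SpawnActor rather than level streaming calls.
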(event `self.BeginMiniGame`
  (bind _returnvalue (`|CreateWidget` "/Game/MiniGameExample/Blueprints/LevelMiniGame/WBP_LevelMiniGameHud.WBP_LevelMiniGameHud_C" (`self.MiniGamePlayerController`)))
  (bind _output_get (set `self.Widget` _returnvalue))
  (`UserWidget.AddToViewport` _output_get 0)
  (bind _returnvalue_2 (`|SpawnActorFromClass` "/Game/MiniGameExample/Blueprints/LevelMiniGame/BP_L_LevelMiniGame.BP_L_LevelMiniGame_C" (`KismetMathLibrary.MakeTransform` (0.0 0.0 1000.0)) "Undefined" "MultiplyWithRoot" null null))
  (set `self.SpawnedLevel` _returnvalue_2)
  (bind _output_get_2 (set `self.Pawn` (`Controller.K2_GetPawn` (`self.MiniGamePlayerController`))))
  (`self.DisableInput` _output_get_2 (`self.MiniGamePlayerController`)))

(event `FinishMiniGame`
  (params (Success :type Boolean))
  (`self.OnFinished` Success)
  (`self.K2_DestroyActor`)
  (`Widget.RemoveFromParent` (`self.Widget`))
  (`self.K2_DestroyActor` (`self.SpawnedLevel`))
  (`self.EnableInput` (`self.Pawn`) (`self.MiniGamePlayerController`)))

(fn `UserConstructionScript`
  (`parent.UserConstructionScript`))