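; Player controller that runs door mini-games, split between server and owning client.
; A request stores the door, sets a waiting flag against overlaps and has the client spawn the mini-game at the door's anchor.
; The client binds the finish event and starts the game, then reports the result to the server, which clears the flag and notifies the door.
; ExitView restores character view, walking, input and hidden cursor.
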(event `RequestMiniGame`
  (params (Door :type "/Game/MiniGameExample/Blueprints/BP_Door Object Reference") (MiniGameClass :type "/Game/MiniGameExample/Blueprints/BP_MiniGameBase Class Reference"))
  (if (not (`self.IsWaitingMinigame`))
    (set `self.Current Door` Door)
    (set `self.IsWaitingMinigame` true)
    (`self.Client_SpawnMiniGame` MiniGameClass (`SceneComponent.K2_GetComponentToWorld` (`/Game/MiniGameExample/Blueprints/BP_Door.MiniGamePosition` (`self.Current Door`))))))

(event `Client_SpawnMiniGame`
  (params (MiniGameClass :type "/Game/MiniGameExample/Blueprints/BP_MiniGameBase Class Reference") (SpawnTransform :type "Transform Structure"))
  (bind _returnvalue (`|SpawnActorFromClass` MiniGameClass SpawnTransform "Undefined" "MultiplyWithRoot" null null))
  (bind _asbp_mini_game_base (cast `/Game/MiniGameExample/Blueprints/BP_MiniGameBase` _returnvalue))
  (add `/Game/MiniGameExample/Blueprints/BP_MiniGameBase.OnFinished` _asbp_mini_game_base (delegate `OnClientEventFinished`))
  (`/Game/MiniGameExample/Blueprints/BP_MiniGameBase.Setup` _asbp_mini_game_base self)
  (`/Game/MiniGameExample/Blueprints/BP_MiniGameBase.BeginMiniGame` _asbp_mini_game_base))

(event `OnClientEventFinished`
  (params (Success :type Boolean))
  (`self.Server_MinigameResult` Success))

(event `Server_MinigameResult`
  (params (Success :type Boolean))
  (bind _current_door (`self.Current Door`))
  (set `self.IsWaitingMinigame` false)
  (`/Engine/EditorBlueprintResources/StandardMacros.IsValid` _current_door
    (:`Is Valid`
      (`/Game/MiniGameExample/Blueprints/BP_Door.OnMiniGameFinished` _current_door Success))))

(event `ExitView`
  (bind _returnvalue (`GameplayStatics.GetNumPlayerControllers`))
  (bind _returnvalue_2 (`GameplayStatics.GetPlayerController` _returnvalue))
  (bind _returnvalue_3 (`GameplayStatics.GetPlayerCharacter` _returnvalue))
  (`/Engine/EditorBlueprintResources/StandardMacros.IsValid` null
    (:`Is Valid`
      (`self.SetViewTargetWithBlend` _returnvalue_2 _returnvalue_3 0.0 "VTBlend_Linear" 0.0 false)
      (`self.EnableInput` _returnvalue_2 _returnvalue_2)
      (`self.ResetIgnoreLookInput` _returnvalue_2)
      (`CharacterMovementComponent.SetMovementMode` (`Character.CharacterMovement` _returnvalue_3) "MOVE_Walking" 0)
      (`WidgetBlueprintLibrary.SetInputMode_GameOnly` _returnvalue_2)
      (set `PlayerController.bShowMouseCursor` false _returnvalue_2))))

(fn `UserConstructionScript`)