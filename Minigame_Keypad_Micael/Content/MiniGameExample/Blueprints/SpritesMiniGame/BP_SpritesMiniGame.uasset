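; A click-the-star sprite mini game actor: clicking the moving Star wins, while clicking the background tilemap or collider loses.
; On begin, it switches the player's view to itself, shows the cursor with click events, and disables pawn input.
; Tick moves the Star at a random starting velocity, bouncing it within fixed Y/Z bounds.
; A click reports the result, then cleanup destroys the actor and restores view and input.
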(event `self.BeginMiniGame`
  (`/Engine/EditorBlueprintResources/StandardMacros.IsValid` (`self.MiniGamePlayerController`)
    (:`Is Valid`
      (`PlayerController.SetViewTargetWithBlend` (`self.MiniGamePlayerController`) self 0.0 "VTBlend_Linear" 0.0 false)
      (set `PlayerController.bShowMouseCursor` true (`self.MiniGamePlayerController`))
      (bind _output_get (set `self.Pawn` (`Controller.K2_GetPawn` (`self.MiniGamePlayerController`))))
      (`self.DisableInput` _output_get (`self.MiniGamePlayerController`))
      (set `PlayerController.bEnableClickEvents` true (`self.MiniGamePlayerController`)))))

(event `CleanUp`
  (`self.K2_DestroyActor`)
  (`/Engine/EditorBlueprintResources/StandardMacros.IsValid` (`self.MiniGamePlayerController`)
    (:`Is Valid`
      (`PlayerController.SetViewTargetWithBlend` (`self.MiniGamePlayerController`) (`self.Pawn`) 0.0 "VTBlend_Linear" 0.0 false)
      (set `PlayerController.bShowMouseCursor` false (`self.MiniGamePlayerController`))
      (`self.EnableInput` (`self.Pawn`) (`self.MiniGamePlayerController`))
      (set `PlayerController.bEnableClickEvents` false (`self.MiniGamePlayerController`)))))

(event `self.Star.OnClicked`
  (params (TouchedComponent :type "PrimitiveComponent Object Reference") (ButtonPressed :type "Key Structure"))
  (`self.OnFinished` true)
  (`self.CleanUp`))

(event `self.BackgroundtileMap.OnClicked`
  (params (TouchedComponent :type "PrimitiveComponent Object Reference") (ButtonPressed :type "Key Structure"))
  (`self.OnFinished` false :!label _label)
  (`self.CleanUp`))

(event `self.backgorund_collider.OnClicked`
  (params (TouchedComponent :type "PrimitiveComponent Object Reference") (ButtonPressed :type "Key Structure"))
  (goto _label))

(event `self.ReceiveBeginPlay`
  (set `self.Velocity` (`KismetMathLibrary.MakeVector` 0.0 (`KismetMathLibrary.RandomFloatInRange` 100.0 200.0) (`KismetMathLibrary.RandomFloatInRange` 100.0 200.0))))

(event `self.ReceiveTick`
  (params (DeltaSeconds :type "Float (single-precision)"))
  (bind (_velocity_x _velocity_y _velocity_z) (`KismetMathLibrary.BreakVector` (`self.Velocity`)))
  (bind (_relativelocation_x _relativelocation_y _relativelocation_z) (`KismetMathLibrary.BreakVector` (`SceneComponent.RelativeLocation` (`self.Star`))))
  (`SceneComponent.K2_AddRelativeLocation` (`self.Star`) (* DeltaSeconds (`self.Velocity`)) false false)
  (set `self.Velocity` (`KismetMathLibrary.MakeVector` 0.0 (`/Game/MiniGameExample/Blueprints/MiniGameFunctionLibrary.BounceFloat` _relativelocation_y _velocity_y -159.0 150.0) (`/Game/MiniGameExample/Blueprints/MiniGameFunctionLibrary.BounceFloat` _relativelocation_z _velocity_z -150.0 150.0))))

(fn `UserConstructionScript`
  (`parent.UserConstructionScript`))