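; BP_Door is a keypad door that players unlock by completing a minigame.
; On the server, interacting closes an open door or requests the minigame through BP_MiniGamePlayerController, with AlreadyInUse blocking concurrent attempts.
; A successful result sets IsOpen, whose RepNotify swaps button materials and plays or reverses a sliding Timeline.
; The right panel and keypad use a cubic ease-out, while the left panel follows the raw curve.
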(event Custom|TryOpenDoor
  (params (PlayerController :type Player%20Controller%20Object%20Reference))
  (bind _asbp_mini_game_player_controller (Utilities|Casting|CastToBP_MiniGamePlayerController PlayerController))
  (Default|RequestMiniGame _asbp_mini_game_player_controller self (Variables|Default|GetMini%20Game%20Class)))

(event Custom|OnMiniGameFinished
  (params (Success :type Boolean))
  (Networking|SwitchHasAuthority
    (:Authority
      (if Success
        (Variables|Default|SetIsOpen true)
        (Variables|Default|SetAlreadyInUse false)
        (Actor|GetAllActorsOfClass "/Game/MiniGameExample/Blueprints/BP_MiniGamePlayerController.BP_MiniGamePlayerController_C")
        (else
          (Variables|Default|SetAlreadyInUse false))))))

(event Custom|PlayCloseAnimation
  (Rendering|Material|SetMaterial (Variables|Default|GetSM_Number0) 0 "/Game/MiniGameExample/Material/MI_ButtonOff.MI_ButtonOff")
  (bind _door_opening_movement (Timeline|Timeline Reverse)
    (:Update
      (Transformation|SetRelativeLocation (Utilities|Array|MakeArray (Variables|Default|GetSM_Number0) (Variables|Default|GetSM_Number1) (Variables|Default|GetSM_Number2) (Variables|Default|GetSM_Number3) (Variables|Default|GetSM_Number4) (Variables|Default|GetSM_Number5) (Variables|Default|GetSM_Number6) (Variables|Default|GetSM_Number7) (Variables|Default|GetSM_Number8) (Variables|Default|GetSM_Visor) (Variables|Default|GetSM_Keypad) (Variables|Default|GetSM_Right_Door)) (Math|Vector|MakeVector (Math|Float|Lerp 0.0 85.0 (|(clamp((1-(pow((1-a),3))))) _door_opening_movement)) 0.0 0.0) false false)
      (Transformation|SetRelativeLocation (Variables|Default|GetSM_Left_Door) (Math|Vector|MakeVector (Math|Float|Lerp 0.0 -7e+01 _door_opening_movement) 0.0 0.0) false false))))

(event Custom|PlayOpenAnimation
  (Rendering|Material|SetMaterial (Variables|Default|GetSM_Number0) 0 "/Game/MiniGameExample/Material/MI_ButtonOn.MI_ButtonOn")
  (bind _door_opening_movement (Timeline|Timeline Play)
    (:Update
      (Transformation|SetRelativeLocation (Utilities|Array|MakeArray (Variables|Default|GetSM_Number0) (Variables|Default|GetSM_Number1) (Variables|Default|GetSM_Number2) (Variables|Default|GetSM_Number3) (Variables|Default|GetSM_Number4) (Variables|Default|GetSM_Number5) (Variables|Default|GetSM_Number6) (Variables|Default|GetSM_Number7) (Variables|Default|GetSM_Number8) (Variables|Default|GetSM_Visor) (Variables|Default|GetSM_Keypad) (Variables|Default|GetSM_Right_Door)) (Math|Vector|MakeVector (Math|Float|Lerp 0.0 85.0 (|(clamp((1-(pow((1-a),3))))) _door_opening_movement)) 0.0 0.0) false false)
      (Transformation|SetRelativeLocation (Variables|Default|GetSM_Left_Door) (Math|Vector|MakeVector (Math|Float|Lerp 0.0 -7e+01 _door_opening_movement) 0.0 0.0) false false))))

(event EventInteract
  (params (PlayerController :type Player%20Controller%20Object%20Reference))
  (Networking|SwitchHasAuthority
    (:Authority
      (if (Variables|Default|GetIsOpen)
        (Variables|Default|SetIsOpen false)
        (elif (Variables|Default|GetAlreadyInUse)
          (Development|PrintString "Puzzle In Use")
          (else
            (CallFunction|TryOpenDoor PlayerController)
            (Variables|Default|SetAlreadyInUse true)))))))

(fn ConstructionScript)

(fn OnRepIsOpen
  (if (Variables|Default|GetIsOpen)
    (CallFunction|PlayOpenAnimation)
    (else
      (CallFunction|PlayCloseAnimation))))

(fn OnRepAlreadyinUse)