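; Keypad minigame actor: a lights-out style puzzle in which the player must switch all nine buttons on.
; BeginMiniGame blends the view to the actor, locks player movement and look, and shows the cursor.
; Clicks line-trace from the cursor, toggling the hit button and its ButtonConfig-linked buttons, swapping on/off materials.
; All buttons on reports success; Q reports failure; both destroy the actor and restore player control.
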(event `self.ReceiveBeginPlay`
  (`parent.ReceiveBeginPlay`)
  (`self.EnableInput` (`self.MiniGamePlayerController`)))

(event `Key|Q`
  (params (Key :type "Key Structure"))
  (:`Pressed`
    (`self.OnFinished` false)
    (`self.K2_DestroyActor`)
    (`self.ExitView`)))

(event `self.BeginMiniGame`
  (bind _minigameplayercontroller (`self.MiniGamePlayerController`))
  (`/Engine/EditorBlueprintResources/StandardMacros.IsValid` (`self.MiniGamePlayerController`)
    (:`Is Valid`
      (`PlayerController.SetViewTargetWithBlend` (`self.MiniGamePlayerController`) self 0.0 "VTBlend_Linear" 0.0 false)
      (`CharacterMovementComponent.DisableMovement` (`Character.CharacterMovement` (`GameplayStatics.GetPlayerCharacter` 0)))
      (`Controller.SetIgnoreLookInput` _minigameplayercontroller true)
      (`KismetSystemLibrary.Delay` 0.5)
      (`self.EnableInput` _minigameplayercontroller)
      (set `PlayerController.bShowMouseCursor` true _minigameplayercontroller))))

(event `Key|LeftMouseButton`
  (params (Key :type "Key Structure"))
  (bind _minigameplayercontroller (`self.MiniGamePlayerController`))
  (bind (_worldlocation _worlddirection _returnvalue) (`PlayerController.DeprojectMousePositionToWorld` _minigameplayercontroller))
  (:`Released`
    (`/Engine/EditorBlueprintResources/StandardMacros.IsValid` _minigameplayercontroller
      (:`Is Valid`
        (if _returnvalue
          (bind (_outhit _returnvalue_2) (`KismetSystemLibrary.LineTraceSingle` :`Start` _worldlocation :`End` (+ _worldlocation (* _worlddirection 150.0)) :`TraceChannel` "TraceTypeQuery1" :`bIgnoreSelf` false))
          (if _returnvalue_2
            (bind (_bblockinghit _binitialoverlap _time _distance _location _impactpoint _normal _impactnormal _physmat _hitactor _hitcomponent) (`GameplayStatics.BreakHitResult` _outhit))
            (`KismetSystemLibrary.PrintString` (`KismetSystemLibrary.GetObjectName` _hitcomponent) false false)
            (bind _asstatic_mesh_component (cast `StaticMeshComponent` _hitcomponent))
            (bind _returnvalue_3 (`KismetArrayLibrary.Array_Find` (`self.Buttons`) _asstatic_mesh_component))
            (`self.ToggleActivation` _returnvalue_3)
            (bind (_value _returnvalue_4) (`BlueprintMapLibrary.Map_Find` (`self.ButtonConfig`) _returnvalue_3))
            (if _returnvalue_4
              (for _array_element (`.Buttons_3_42388AF848B8D3B11497D0AB9C398279` (break `/Game/MiniGameExample/Struct/S_ButtonsToActivate` _value))
                (`self.ToggleActivation` _array_element)))
            (bind _success (`self.CheckAnswers`))
            (if _success
              (`self.OnFinished` true)
              (`self.MinigameCompleted`)
              (`self.K2_DestroyActor`)
              (`self.ExitView`))))))))

(event `ExitView`
  (bind _returnvalue (`GameplayStatics.GetPlayerCharacter` 0))
  (bind _minigameplayercontroller (`self.MiniGamePlayerController`))
  (`PlayerController.SetViewTargetWithBlend` _minigameplayercontroller _returnvalue 0.0 "VTBlend_Linear" 0.0 false)
  (`self.DisableInput` _minigameplayercontroller)
  (`Controller.ResetIgnoreLookInput` _minigameplayercontroller)
  (`CharacterMovementComponent.SetMovementMode` (`Character.CharacterMovement` _returnvalue) "MOVE_Walking" 0)
  (`WidgetBlueprintLibrary.SetInputMode_GameOnly` _minigameplayercontroller)
  (set `PlayerController.bShowMouseCursor` false _minigameplayercontroller))

(event `MinigameCompleted`)

(fn `CheckAnswers`
  (returns (Success :type Boolean))
  (if (== (`KismetArrayLibrary.Array_Length` (`self.Buttons`)) (`KismetArrayLibrary.Array_Length` (`self.ButtonActivationState`)))
    (for _array_element (`self.ButtonActivationState`)
      (if (not _array_element)
        (return false)))
    (return true)
    (else
      (`KismetSystemLibrary.PrintString` "Error!"))))

(fn `ToggleActivation`
  (params (`Button Index` :type Integer))
  (bind _buttonactivationstate (`self.ButtonActivationState`))
  (bind _output (`|GetArrayItem` (`self.Buttons`) `Button Index`))
  (`KismetArrayLibrary.Array_Set` _buttonactivationstate `Button Index` (not (`|GetArrayItem` _buttonactivationstate `Button Index`)))
  (`KismetSystemLibrary.PrintString` (`KismetSystemLibrary.GetObjectName` _output) false false)
  (if (`|GetArrayItem` _buttonactivationstate `Button Index`)
    (`/Engine/EditorBlueprintResources/StandardMacros.IsValid` _output
      (:`Is Valid`
        (`PrimitiveComponent.SetMaterial` _output 0 "/Game/MiniGameExample/Material/M_ButtonOn.M_ButtonOn")))
    (else
      (`/Engine/EditorBlueprintResources/StandardMacros.IsValid` _output
        (:`Is Valid`
          (`PrimitiveComponent.SetMaterial` _output 0 "/Game/MiniGameExample/Material/M_ButtonOff.M_ButtonOff"))))))

(fn `UserConstructionScript`
  (set `self.Buttons` (`|MakeArray` (`self.SM_Number0`) (`self.SM_Number1`) (`self.SM_Number2`) (`self.SM_Number3`) (`self.SM_Number4`) (`self.SM_Number5`) (`self.SM_Number6`) (`self.SM_Number7`) (`self.SM_Number8`))))