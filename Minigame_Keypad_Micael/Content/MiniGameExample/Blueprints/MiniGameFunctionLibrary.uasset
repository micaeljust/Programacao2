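; Blueprint function library for the mini game example, providing a helper that bounces a value between bounds.
; BounceFloat takes a position, its current speed and min and max limits, and returns the speed to use next.
; Past the maximum it returns a negative speed, below the minimum a positive one, otherwise the speed unchanged.
; Forcing the sign from the absolute speed keeps an out-of-range value heading back inside without flipping repeatedly.
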(fn `BounceFloat`
  (params (pos :type "Float (double-precision)") (currentSpeed :type "Float (double-precision)") (minPos :type "Float (double-precision)") (maxPos :type "Float (double-precision)"))
  (returns (Speed :type "Float (double-precision)"))
  (if (> (`local.pos`) (`local.maxPos`))
    (return (* (`KismetMathLibrary.Abs` (`local.currentSpeed`)) -1.0))
    (elif (< (`local.pos`) (`local.minPos`))
      (return (`KismetMathLibrary.Abs` (`local.currentSpeed`)))
      (else
        (return (`local.currentSpeed`))))))