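; BP_HudMiniGame is an example mini-game actor that runs entirely as a HUD widget.
; On begin, it creates WBP_HudMiniGame for the mini-game controller, adds it to the viewport and switches to UI-only input with a visible cursor.
; When the widget's finished event fires, it passes the success result on through CallOnFinished, removes the widget, destroys itself and restores game-only input with a hidden cursor.
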(event `self.BeginMiniGame`
  (`WidgetBlueprintLibrary.SetInputMode_UIOnlyEx` (`self.MiniGamePlayerController`) null)
  (bind _returnvalue (`|CreateWidget` "/Game/MiniGameExample/Blueprints/HudMiniGame/WBP_HudMiniGame.WBP_HudMiniGame_C" (`self.MiniGamePlayerController`)))
  (bind _output_get (set `self.Widget` _returnvalue))
  (add `/Game/MiniGameExample/Blueprints/HudMiniGame/WBP_HudMiniGame.OnFinished` _output_get (delegate `OnWidgetFinished`))
  (`UserWidget.AddToViewport` (`self.Widget`) 0)
  (set `PlayerController.bShowMouseCursor` true (`self.MiniGamePlayerController`)))

(event `OnWidgetFinished`
  (params (Success :type Boolean))
  (`self.OnFinished` Success)
  (`Widget.RemoveFromParent` (`self.Widget`))
  (`self.K2_DestroyActor`)
  (`WidgetBlueprintLibrary.SetInputMode_GameOnly` (`self.MiniGamePlayerController`))
  (set `PlayerController.bShowMouseCursor` false (`self.MiniGamePlayerController`)))

(fn `UserConstructionScript`
  (`parent.UserConstructionScript`))